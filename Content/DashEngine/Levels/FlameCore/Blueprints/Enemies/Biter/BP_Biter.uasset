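; Biter enemy that spots the Dash player through PawnSensing and closes in to attack.
; Each sighting yaws the capsule toward the player, and a DoOnce starts a single AI move that calls Attack on arrival within range.
; Attack only sets the animation state and ReadyToAttack flag, with debug prints here and on Tick.
; The NearCollision overlap is empty, leaving its proximity attack logic disconnected.
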(event OnSeePawn(PawnSensing)
  (params (Pawn :type Pawn%20Object%20Reference))
  (bind _asdash_player_pawn (Utilities|Casting|CastToDashPlayerPawn Pawn))
  (Transformation|SetRelativeRotation (Variables|Collision|GetCapsuleComponent) (Math|Rotator|MakeRotator 0.0 0.0 (.yaw (CallFunction|GetLookatRotation self _asdash_player_pawn))) false false)
  (if (not (Variables|Default|GetReadyToAttack?))
    (Utilities|FlowControl|DoOnce false
      (:Completed
        (AI|AIMoveTo self "0, 0, 0" _asdash_player_pawn 8e+02 false
          (:OnSuccess
            (CallFunction|Attack)
            (Development|PrintString "success")))))))

(event OnComponentBeginOverlap(NearCollision)
  (params (OverlappedComponent :type Primitive%20Component%20Object%20Reference) (OtherActor :type Actor%20Object%20Reference) (OtherComp :type Primitive%20Component%20Object%20Reference) (OtherBodyIndex :type Integer) (bFromSweep :type Boolean) (SweepResult :type Hit%20Result%20Structure%20%28by%20ref%29)))

(event Custom|Attack
  (Variables|Default|SetAnimState "NewEnumerator0")
  (Variables|Default|SetReadyToAttack? true)
  (Development|PrintString "attack"))

(event EventBeginPlay)

(event EventTick
  (params (DeltaSeconds :type Float%20%28single-precision%29))
  (Development|PrintString (Utilities|String|EnumtoString (Variables|Default|GetAnimState))))

(fn ConstructionScript)