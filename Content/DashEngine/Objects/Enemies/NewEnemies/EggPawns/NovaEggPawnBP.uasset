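; Nova Egg Pawn enemy that spots the player, closes in and punches, driving an AnimState enum as it goes.
; Pawn sensing triggers a short reaction delay, then AI MoveTo chases the player and flags OnTarget on arrival.
; A later sighting while on target calls Punch, which clears the flag and is gated by a DoOnce that resets after AttackCooldown.
; Tick restores the default anim state when horizontally stationary, off target and not reacting.
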(event OnSeePawn(PawnSensing)
  (params (Pawn :type Pawn%20Object%20Reference))
  (bind _asdash_player_pawn (Utilities|Casting|CastToDashPlayerPawn Pawn))
  (if (Variables|Default|GetOnTarget)
    (CallFunction|Punch)
    (else
      (Variables|Default|SetAnimState "NewEnumerator2")
      (Utilities|FlowControl|Delay 0.9)
      (Variables|Default|SetAnimState "NewEnumerator1")
      (AI|AIMoveTo self "0, 0, 0" _asdash_player_pawn 3e+02 true
        (:OnSuccess
          (Variables|Default|SetOnTarget true))))))

(event Custom|Punch
  (Utilities|FlowControl|DoOnce false :!label _label
    (:Completed
      (Variables|Default|SetAnimState "NewEnumerator3")
      (Variables|Default|SetOnTarget false)
      (Utilities|FlowControl|Delay (Variables|Default|GetAttackCooldown))
      (goto _label Reset))))

(event EventTick
  (params (DeltaSeconds :type Float%20%28single-precision%29))
  (bind _returnvalue (Transformation|GetVelocity))
  (if (Math|Boolean|ANDBoolean (== (.x _returnvalue) 0.0) (== (.y _returnvalue) 0.0) (not (Utilities|Enum|Equal(Enum) (Variables|Default|GetAnimState) "NewEnumerator2")) (not (Variables|Default|GetOnTarget)))
    (Variables|Default|SetAnimState "NewEnumerator0")))

(fn ConstructionScript)